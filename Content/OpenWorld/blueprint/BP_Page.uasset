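; BP_Page is an interactable page object, represented by a Cube component, that triggers an action on a linked PageActor.
; BecomeApply swaps the cube's material to Mat and caches the previous one, which OutOfApply restores.
; Interact hides the cube, waits briefly, then calls Act through BPI_PageActorAction and destroys itself, but only if PageActor implements that interface.
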(event EventBeginPlay)

(event Collision|EventActorBeginOverlap
  (params (OtherActor :type Actor%20Object%20Reference)))

(event EventTick
  (params (DeltaSeconds :type Float%20%28single-precision%29)))

(event EventBecomeApply
  (bind _cube (Variables|Default|GetCube))
  (Variables|Default|SetPrevMat (Rendering|Material|GetMaterial _cube 0))
  (Rendering|Material|SetMaterial _cube 0 (Variables|Default|Getmat)))

(event EventInteract
  (params (InteractMesh :type Mesh%20Component%20Object%20Reference))
  (Development|SetHiddeninGame (Variables|Default|GetCube) true false)
  (Utilities|FlowControl|Delay 3.0)
  (if (Utilities|DoesObjectImplementInterface (Variables|Default|GetPageActor) "/Game/OpenWorld/BPI_PageActorAction.BPI_PageActorAction_C")
    (Class|BPIPageActorAction|Act(Message) (Variables|Default|GetPageActor))
    (Actor|DestroyActor)))

(event EventOutOfApply
  (Rendering|Material|SetMaterial (Variables|Default|GetCube) 0 (Variables|Default|GetPrevMat)))

(fn ConstructionScript)