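; BP_Boat1 is an interactable boat actor that attaches to whatever mesh interacts with it.
; Its Plane component starts hidden with physics off, and the Act event turns physics on without unhiding it.
; Interact snaps the attachment to the mesh's ik_foot_root socket, calls OutOfApply and sets IsActing.
; BecomeApply and OutOfApply are empty, leaving the material-swap nodes disconnected.
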(event EventBeginPlay
  (bind _plane (Variables|Default|GetPlane))
  (Development|SetHiddeninGame _plane true false)
  (Physics|SetSimulatePhysics _plane false))

(event Collision|EventActorBeginOverlap
  (params (OtherActor :type Actor%20Object%20Reference)))

(event EventTick
  (params (DeltaSeconds :type Float%20%28single-precision%29)))

(event EventBecomeApply)

(event EventInteract
  (params (InteractMesh :type Mesh%20Component%20Object%20Reference))
  (Transformation|AttachComponentToComponent InteractMesh "ik_foot_root" "SnapToTarget" "KeepRelative" "KeepRelative" true)
  (CallFunction|OutOfApply)
  (Variables|Default|SetIsActing true))

(event EventOutOfApply)

(event EventAct
  (Physics|SetSimulatePhysics (Variables|Default|GetPlane) true))

(fn ConstructionScript)