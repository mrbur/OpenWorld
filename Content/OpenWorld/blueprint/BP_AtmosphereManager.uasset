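; Open-world atmosphere manager that rotates a directional light as a sun cycle and adjusts exponential height fog to match.
; SunEvent steps and wraps the angle, then calls a fog event that shows, thickens or hides and resets fog by angle range.
; The thinning range is nested inside the thickening range, so they barely overlap.
; BeginPlay is empty; the fog lookup and looping timer setup are disconnected, so nothing here starts the cycle.
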(event Custom|SunEvent
  (if (> (Variables|Default|Getrotation) 2.7e+02)
    (Variables|Default|Setrotation -9e+01)
    (else
      (bind _output_get (Variables|Default|Setrotation (+ (Variables|Default|Getrotation) 0.3)))))
  (Transformation|SetActorRotation (Variables|Default|GetDirectionalLight) (Math|Rotator|MakeRotator 0.0 _output_get 0.0))
  (CallFunction|CustomEvent0))

(event Custom|CustomEvent_0
  (bind _fog (Variables|Default|GetFog))
  (bind _component (Variables|/Script/Engine.ExponentialHeightFog|GetComponent _fog))
  (if (Math|Float|InRange(Float) (Variables|Default|Getrotation) -7.0 1.8e+02)
    (if (Math|Float|InRange(Float) (Variables|Default|Getrotation) 1.8e+02 195.0)
      (bind _output_get (Variables|Default|SetFogDensity (/ (Variables|Default|GetFogDensity) 1.1)))
      (Class|ExponentialHeightFogComponent|SetFogDensity (Variables|/Script/Engine.ExponentialHeightFog|GetComponent (Variables|Default|GetFog)) _output_get)
      (else
        (bind _output_get_2 (Variables|Default|SetFogDensity (* (Variables|Default|GetFogDensity) 1.007)))
        (Class|ExponentialHeightFogComponent|SetFogDensity (Variables|/Script/Engine.ExponentialHeightFog|GetComponent (Variables|Default|GetFog)) _output_get_2)))
    (elif (Math|Float|InRange(Float) (Variables|Default|Getrotation) -8.0 -7.0)
      (Rendering|SetVisibility (Variables|/Script/Engine.ExponentialHeightFog|GetComponent _fog) true false)
      (elif (Math|Float|InRange(Float) (Variables|Default|Getrotation) 195.0 197.0)
        (Rendering|SetVisibility _component false false)
        (bind _output_get_3 (Variables|Default|SetFogDensity 0.001))
        (Class|ExponentialHeightFogComponent|SetFogDensity _component _output_get_3)))))

(event EventBeginPlay)

(fn ConstructionScript)