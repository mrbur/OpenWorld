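; BP_Boat is an interactable boat actor that attaches to the interacting mesh.
; Its Cube starts hidden without physics until Act reveals it and enables simulation.
; BecomeApply and OutOfApply highlight and restore the Cube by swapping and caching its material.
; Interact snaps the boat to the mesh's ik_foot_root socket, restores the material and sets IsActing, which blocks further highlighting.
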(event EventBeginPlay
  (Development|SetHiddeninGame (Variables|Default|GetCube) true false)
  (Physics|SetSimulatePhysics (Variables|Default|GetCube) false))

(event Collision|EventActorBeginOverlap
  (params (OtherActor :type Actor%20Object%20Reference)))

(event EventTick
  (params (DeltaSeconds :type Float%20%28single-precision%29)))

(event EventBecomeApply
  (bind _cube (Variables|Default|GetCube))
  (if (not (Variables|Default|GetIsActing))
    (Variables|Default|SetPrevMat (Rendering|Material|GetMaterial _cube 0))
    (Rendering|Material|SetMaterial _cube 0 (Variables|Default|Getmat))))

(event EventInteract
  (params (InteractMesh :type Mesh%20Component%20Object%20Reference))
  (Transformation|AttachComponentToComponent InteractMesh "ik_foot_root" "SnapToTarget" "KeepRelative" "KeepRelative" true)
  (CallFunction|OutOfApply)
  (Variables|Default|SetIsActing true))

(event EventOutOfApply
  (Rendering|Material|SetMaterial (Variables|Default|GetCube) 0 (Variables|Default|GetPrevMat)))

(event EventAct
  (Development|SetHiddeninGame (Variables|Default|GetCube) false false)
  (Physics|SetSimulatePhysics (Variables|Default|GetCube) true))

(fn ConstructionScript)