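; Animal character blueprint for a crow that moves away along its arrow's heading with an upward component.
; Two trigger boxes detect the player: Box sets a Near flag, while Box1 sets Close and enables actor tick.
; Each tick adds movement input from the arrow's forward X and Y, using mesh world height plus an offset as Z.
; Neither flag is read or cleared in these graphs.
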(event OnComponentBeginOverlap(Box)
  (params (OverlappedComponent :type Primitive%20Component%20Object%20Reference) (OtherActor :type Actor%20Object%20Reference) (OtherComp :type Primitive%20Component%20Object%20Reference) (OtherBodyIndex :type Integer) (bFromSweep :type Boolean) (SweepResult :type Hit%20Result%20Structure%20%28by%20ref%29))
  (Utilities|Casting|CastToBP_CharacterPlayer OtherActor)
  (Variables|Default|Setnear true))

(event OnComponentBeginOverlap(Box1)
  (params (OverlappedComponent :type Primitive%20Component%20Object%20Reference) (OtherActor :type Actor%20Object%20Reference) (OtherComp :type Primitive%20Component%20Object%20Reference) (OtherBodyIndex :type Integer) (bFromSweep :type Boolean) (SweepResult :type Hit%20Result%20Structure%20%28by%20ref%29))
  (Utilities|Casting|CastToBP_CharacterPlayer OtherActor)
  (Variables|Default|Setclose true)
  (Actor|Tick|SetActorTickEnabled true))

(event OnComponentEndOverlap(Box)
  (params (OverlappedComponent :type Primitive%20Component%20Object%20Reference) (OtherActor :type Actor%20Object%20Reference) (OtherComp :type Primitive%20Component%20Object%20Reference) (OtherBodyIndex :type Integer)))

(event EventBeginPlay)

(event Collision|EventActorBeginOverlap
  (params (OtherActor :type Actor%20Object%20Reference)))

(event EventTick
  (params (DeltaSeconds :type Float%20%28single-precision%29))
  (bind _arrowcomponent (Variables|Default|GetArrowComponent))
  (bind _returnvalue (Math|Vector|GetForwardVector _arrowcomponent))
  (Pawn|Input|AddMovementInput (Math|Vector|MakeVector (.x _returnvalue) (.y _returnvalue) (+ (.z (Transformation|GetWorldLocation (Variables|Character|GetMesh))) 2.0)) 1.0 false))

(fn ConstructionScript)