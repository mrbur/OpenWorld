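; BP_Character is the open-world player character, handling movement, camera look and the pause menu.
; Axis inputs move it along the control rotation's yaw and feed controller pitch and yaw.
; The QPause action drives a FlipFlop that pauses or unpauses the game, creating or removing W_PauseWidget and switching cursor and input mode.
; A Resume event feeds the same FlipFlop, keeping the toggle in sync.
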(event Custom|Resume
  (bind _returnvalue (Game|GetPlayerController 0))
  (bind _returnvalue_2 (Game|GetPlayerController 0))
  (Utilities|FlowControl|FlipFlop
    (:A
      (Game|SetGamePaused true)
      (bind _returnvalue_3 (UserInterface|CreateWidget "/Game/OpenWorld/widget/W_PauseWidget.W_PauseWidget_C"))
      (bind _output_get (Variables|Default|SetPauseWidget _returnvalue_3))
      (UserInterface|Viewport|AddtoPlayerScreen _output_get)
      (Variables|/Script/Engine.PlayerController|SetbShowMouseCursor _returnvalue true)
      (Input|SetInputModeGameandUI _returnvalue (Variables|Default|GetPauseWidget) "DoNotLock" true))
    (:B
      (Game|SetGamePaused false)
      (Widget|RemovefromParent (Variables|Default|GetPauseWidget))
      (Variables|/Script/Engine.PlayerController|SetbShowMouseCursor _returnvalue_2 false)
      (Input|SetInputModeGameOnly _returnvalue_2))))

(event EventBeginPlay)

(event Collision|EventActorBeginOverlap
  (params (OtherActor :type Actor%20Object%20Reference)))

(event EventTick
  (params (DeltaSeconds :type Float%20%28single-precision%29)))

(event Input|ActionEvents|InputActionQPause
  (params (Key :type Key%20Structure :default "None"))
  (bind _returnvalue (Game|GetPlayerController 0))
  (bind _returnvalue_2 (Game|GetPlayerController 0))
  (:Pressed
    (Utilities|FlowControl|FlipFlop
      (:A
        (Game|SetGamePaused true)
        (bind _returnvalue_3 (UserInterface|CreateWidget "/Game/OpenWorld/widget/W_PauseWidget.W_PauseWidget_C"))
        (bind _output_get (Variables|Default|SetPauseWidget _returnvalue_3))
        (UserInterface|Viewport|AddtoPlayerScreen _output_get)
        (Variables|/Script/Engine.PlayerController|SetbShowMouseCursor _returnvalue true)
        (Input|SetInputModeGameandUI _returnvalue (Variables|Default|GetPauseWidget) "DoNotLock" true))
      (:B
        (Game|SetGamePaused false)
        (Widget|RemovefromParent (Variables|Default|GetPauseWidget))
        (Variables|/Script/Engine.PlayerController|SetbShowMouseCursor _returnvalue_2 false)
        (Input|SetInputModeGameOnly _returnvalue_2)))))

(event Input|AxisEvents|InputAxisMoveForvard
  (params (AxisValue :type Float%20%28single-precision%29))
  (Pawn|Input|AddMovementInput (Math|Vector|GetForwardVector (Math|Rotator|MakeRotator 0.0 0.0 (.yaw (Pawn|GetControlRotation :!class /Script/Engine.Pawn)))) AxisValue false))

(event Input|AxisEvents|InputAxisMoveRight
  (params (AxisValue :type Float%20%28single-precision%29))
  (Pawn|Input|AddMovementInput (Math|Vector|GetRightVector (Math|Rotator|MakeRotator 0.0 0.0 (.yaw (Pawn|GetControlRotation :!class /Script/Engine.Pawn)))) AxisValue false))

(event Input|AxisEvents|InputAxisLookUp
  (params (AxisValue :type Float%20%28single-precision%29))
  (Pawn|Input|AddControllerPitchInput AxisValue))

(event Input|AxisEvents|InputAxisTurn
  (params (AxisValue :type Float%20%28single-precision%29))
  (Pawn|Input|AddControllerYawInput AxisValue))

(fn ConstructionScript)